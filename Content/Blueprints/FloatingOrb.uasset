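; FloatingOrb is an actor Blueprint that bobs gently up and down around the spot where it starts.
; BeginPlay caches the starting transform, and Tick accumulates elapsed time to drive a sine offset on Z while X and Y stay at their starting values.
; The overlap event and construction script are empty, so the motion is its only behavior.
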(event EventBeginPlay
  (Variables|Default|SetStartTransform (Transformation|GetActorTransform)))

(event Collision|EventActorBeginOverlap
  (params (OtherActor :type Actor%20Object%20Reference)))

(event EventTick
  (params (DeltaSeconds :type Float%20%28single-precision%29))
  (bind _starttransform (Variables|Default|GetStartTransform))
  ;[1 1 1] Track time elapsed
  (bind _output_get (Variables|Default|SetCuumulatedTime (+ DeltaSeconds (Variables|Default|GetCuumulatedTime))))
  (Transformation|SetActorLocation (Math|Vector|MakeVector (.x (.location _starttransform)) (.y (.location _starttransform)) (+ (* (Math|Trig|Sin(Radians) _output_get) 5.0) (.z (.location _starttransform)))) false false))

(fn ConstructionScript)